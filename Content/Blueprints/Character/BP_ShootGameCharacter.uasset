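; Player character Blueprint for a shooter, mapping Enhanced Input actions to character abilities.
; Jump and aim follow press and release, while crouch toggles on each press.
; Pick calls EquipWeapon and fire calls Fire; these functions and Aim are not defined here, so the graph serves only as input wiring.
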(event `EnhancedInput|/Game/Blueprints/Input/InputAcion/IA_Jump`
  (params (ActionValue :type Boolean) (ElapsedSeconds :type "Float (double-precision)") (TriggeredSeconds :type "Float (double-precision)") (InputAction :type "InputAction Object Reference" :default "/Game/Blueprints/Input/InputAcion/IA_Jump.IA_Jump"))
  (:`Started`
    (`self.Jump`))
  (:`Completed`
    (`self.StopJumping`)))

(event `EnhancedInput|/Game/Blueprints/Input/InputAcion/IA_Crouch`
  (params (ActionValue :type Boolean) (ElapsedSeconds :type "Float (double-precision)") (TriggeredSeconds :type "Float (double-precision)") (InputAction :type "InputAction Object Reference" :default "/Game/Blueprints/Input/InputAcion/IA_Crouch.IA_Crouch"))
  (:`Started`
    (if (`self.bIsCrouched`)
      (`self.UnCrouch`)
      (else
        (`self.Crouch`)))))

(event `EnhancedInput|/Game/Blueprints/Input/InputAcion/IA_Pick`
  (params (ActionValue :type Boolean) (ElapsedSeconds :type "Float (double-precision)") (TriggeredSeconds :type "Float (double-precision)") (InputAction :type "InputAction Object Reference" :default "/Game/Blueprints/Input/InputAcion/IA_Pick.IA_Pick"))
  (:`Started`
    (`self.EquipWeapon`)))

(event `EnhancedInput|/Game/Blueprints/Input/InputAcion/IA_Aim`
  (params (ActionValue :type Boolean) (ElapsedSeconds :type "Float (double-precision)") (TriggeredSeconds :type "Float (double-precision)") (InputAction :type "InputAction Object Reference" :default "/Game/Blueprints/Input/InputAcion/IA_Aim.IA_Aim"))
  (:`Started`
    (`self.Aim` true))
  (:`Completed`
    (`self.Aim` false)))

(event `EnhancedInput|/Game/Blueprints/Input/InputAcion/IA_Fire`
  (params (ActionValue :type Boolean) (ElapsedSeconds :type "Float (double-precision)") (TriggeredSeconds :type "Float (double-precision)") (InputAction :type "InputAction Object Reference" :default "/Game/Blueprints/Input/InputAcion/IA_Fire.IA_Fire"))
  (:`Triggered`
    (`self.Fire`)))

(fn `UserConstructionScript`)